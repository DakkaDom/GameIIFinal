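; Health component that tracks current health and death state, with debug messages printed to screen.
; BeginPlay fills health to the maximum, and ApplyDamage subtracts clamped damage until health reaches zero and sets the dead flag.
; A separate Die event destroys player character 0 rather than the owning actor, and nothing in this file calls it.
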(event `Die`
  (`Actor.K2_DestroyActor` (`GameplayStatics.GetPlayerCharacter` 0)))

(event `self.ReceiveBeginPlay`
  (bind _output_get (set `self.CurrentHealth` (`self.MaxHealth`)))
  (set `self.IsDead` false)
  (`KismetSystemLibrary.PrintString` (`KismetStringLibrary.Conv_DoubleToString` _output_get)))

(fn `ApplyDamage`
  (params (Damage :type "Float (double-precision)"))
  (`KismetSystemLibrary.PrintString` "Damage Taken")
  (if (not (`self.IsDead`))
    (bind _output_get (set `self.CurrentHealth` (`KismetMathLibrary.FClamp` (- (`self.CurrentHealth`) Damage) 0.0 (`self.MaxHealth`))))
    (`KismetSystemLibrary.PrintString` (`KismetStringLibrary.Conv_DoubleToString` _output_get))
    (if (<= (`self.CurrentHealth`) 0.0)
      (set `self.IsDead` true)
      (`KismetSystemLibrary.PrintString` "You Died"))))