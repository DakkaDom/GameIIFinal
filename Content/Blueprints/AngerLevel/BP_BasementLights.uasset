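; Basement light actor in the Anger level that switches on when the player completes the level.
; Tick polls LevelComplete on the player's BP_ThirdPersonCharacter, then after a short Delay shows the point light and swaps the bulb's material.
; It also finds BP_BasementWall by class and makes its wall mesh visible and collidable.
; No latch stops this, so the sequence repeats while the flag stays true.
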(event `self.ReceiveTick`
  (params (DeltaSeconds :type "Float (single-precision)"))
  (bind _asbp_third_person_character (cast `/Game/ThirdPerson/Blueprints/BP_ThirdPersonCharacter` (`GameplayStatics.GetPlayerCharacter` 0)))
  (if (`/Game/ThirdPerson/Blueprints/BP_ThirdPersonCharacter.LevelComplete` _asbp_third_person_character)
    (`KismetSystemLibrary.Delay` 3.0)
    (`SceneComponent.SetVisibility` (`self.PointLight`) true false)
    (`PrimitiveComponent.SetMaterial` (`self.SM_Prop_Light_Bulb_01`) 0 "/Game/PolygonHorrorMansion/Materials/Alts/M_PolygonHorrorMansion_Mat_01_A.M_PolygonHorrorMansion_Mat_01_A")
    (bind _returnvalue (`GameplayStatics.GetActorOfClass` "/Game/Blueprints/AngerLevel/BP_BasementWall.BP_BasementWall_C"))
    (bind _sm_bld_base_wall_01 (`/Game/Blueprints/AngerLevel/BP_BasementWall.SM_Bld_Base_Wall_01` _returnvalue))
    (`SceneComponent.SetVisibility` _sm_bld_base_wall_01 true false)
    (`PrimitiveComponent.SetCollisionEnabled` _sm_bld_base_wall_01 "QueryAndPhysics")))

(fn `UserConstructionScript`)