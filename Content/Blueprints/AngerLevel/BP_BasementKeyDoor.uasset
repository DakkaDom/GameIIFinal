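; BP_BasementKeyDoor is a basement door that opens only when the player character has the basement key.
; OpenDoorWithButton finds BP_ThirdPersonCharacter and checks HasBasementKey.
; With the key, a timeline rotates the door mesh 90 degrees and a DoOnce plays the creak sound a single time.
; Without it, a locked sound plays and the character's key-needed widget shows for two seconds.
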(event `OpenDoorWithButton`
  (bind _returnvalue (`GameplayStatics.GetActorOfClass` "/Game/ThirdPerson/Blueprints/BP_ThirdPersonCharacter.BP_ThirdPersonCharacter_C"))
  (bind _asbp_third_person_character (cast `/Game/ThirdPerson/Blueprints/BP_ThirdPersonCharacter` _returnvalue))
  (if (`/Game/ThirdPerson/Blueprints/BP_ThirdPersonCharacter.HasBasementKey` _asbp_third_person_character)
    (bind (_direction _doorfloat) (`Timeline|Timeline`)
      (:`Update`
        (`SceneComponent.K2_SetRelativeRotation` (`self.SM_BasementDoor`) (`KismetMathLibrary.RLerp` (struct) (struct :`Yaw` -90.0) _doorfloat) false false)
        (`/Engine/EditorBlueprintResources/StandardMacros.DoOnce` false
          (:`Completed`
            (`GameplayStatics.PlaySoundAtLocation` "/Game/Audio/Door_Creak.Door_Creak" (0.0 0.0 0.0) (struct) 1.0 1.0 0.0 null null null null)))))
    (else
      (`GameplayStatics.PlaySoundAtLocation` "/Game/Audio/Locked_Door.Locked_Door" (0.0 0.0 0.0) (struct) 1.0 1.0 0.0 null null null null)
      (bind _keyneededwidget (`/Game/ThirdPerson/Blueprints/BP_ThirdPersonCharacter.KeyNeededWidget` _asbp_third_person_character))
      (`Widget.SetVisibility` _keyneededwidget "Visible")
      (`KismetSystemLibrary.Delay` 2.0)
      (`Widget.SetVisibility` _keyneededwidget "Hidden"))))

(fn `UserConstructionScript`)