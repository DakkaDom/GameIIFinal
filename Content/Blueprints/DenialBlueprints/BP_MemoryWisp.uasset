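; BP_MemoryWisp is a collectible wisp that the player picks up by interacting while in range.
; Collision box overlaps with BP_ThirdPersonCharacter toggle the range flag and print debug greetings.
; On collection it decrements RemainingWisps on BP_WispManager, destroys itself, prints the remaining count and increments its own WispsCollected.
; OpenDoor checks that count but its branches are empty, and FloatAround is an empty stub.
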(event `self.ReceiveBeginPlay`)

(event `OpenDoor`
  (`|ExecutionSequence`
    (:`then_0`
      (if (== (`self.WispsCollected`) 1)
        _))
    (:`then_1`
      (if (== (`self.WispsCollected`) 2)
        _))
    (:`then_2`
      (if (== (`self.WispsCollected`) 3)
        _))))

(event `/Game/Blueprints/BlueprintInterfaces/BPI_Interact.Interact`
  (params (PlayerCharacter :type "/Game/ThirdPerson/Blueprints/BP_ThirdPersonCharacter Object Reference"))
  (`self.GetCollected`))

(event `FloatAround`)

(event `GetCollected`
  (if (`self.WithinRange`)
    (bind _returnvalue (`GameplayStatics.GetActorOfClass` "/Game/Blueprints/DenialBlueprints/BP_WispManager.BP_WispManager_C"))
    (bind _result (`/Engine/EditorBlueprintResources/StandardMacros.DecrementInt` (`/Game/Blueprints/DenialBlueprints/BP_WispManager.RemainingWisps` _returnvalue))
      (:`  `
        (`self.K2_DestroyActor`)
        (`KismetSystemLibrary.PrintText` (`|FormatText` "There are {number} wisps in the level" _result))
        (`/Engine/EditorBlueprintResources/StandardMacros.IncrementInt` (`self.WispsCollected`))))))

(event `self.CollisionBox.OnComponentBeginOverlap`
  (params (OverlappedComponent :type "PrimitiveComponent Object Reference") (OtherActor :type "Actor Object Reference") (OtherComp :type "PrimitiveComponent Object Reference") (OtherBodyIndex :type Integer) (bFromSweep :type Boolean) (SweepResult :type "HitResult Structure (by ref)"))
  (cast `/Game/ThirdPerson/Blueprints/BP_ThirdPersonCharacter` OtherActor)
  (set `self.WithinRange` true)
  (`KismetSystemLibrary.PrintString` "Wisp Hello"))

(event `self.CollisionBox.OnComponentEndOverlap`
  (params (OverlappedComponent :type "PrimitiveComponent Object Reference") (OtherActor :type "Actor Object Reference") (OtherComp :type "PrimitiveComponent Object Reference") (OtherBodyIndex :type Integer))
  (cast `/Game/ThirdPerson/Blueprints/BP_ThirdPersonCharacter` OtherActor)
  (set `self.WithinRange` false)
  (`KismetSystemLibrary.PrintString` "Wisp Bye"))

(fn `UserConstructionScript`)