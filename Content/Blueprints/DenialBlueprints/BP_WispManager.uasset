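; BP_WispManager tracks the memory wisps in a level and reveals the Denial NPC once none remain.
; On BeginPlay it gathers all BP_MemoryWisp actors, stores their count as RemainingWisps and prints it.
; Its SpawnGhost event calls Appear on the existing BP_Npc_Denial when that count is below one.
; The count is not decremented within this Blueprint.
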(event `self.ReceiveBeginPlay`
  (bind _outactors (`GameplayStatics.GetAllActorsOfClass` "/Game/Blueprints/DenialBlueprints/BP_MemoryWisp.BP_MemoryWisp_C"))
  (bind _output_get (set `self.TotalWisps` _outactors))
  (bind _output_get_2 (set `self.RemainingWisps` (`KismetArrayLibrary.Array_Length` _output_get)))
  (`KismetSystemLibrary.PrintText` (`|FormatText` "There are {number} wisps in the level" _output_get_2)))

(event `SpawnGhost`
  (if (< (`self.RemainingWisps`) 1)
    (bind _returnvalue (`GameplayStatics.GetActorOfClass` "/Game/Blueprints/BP_Npc_Denial.BP_Npc_Denial_C"))
    (`/Game/Blueprints/BP_Npc_Denial.Appear` _returnvalue)))

(fn `UserConstructionScript`)