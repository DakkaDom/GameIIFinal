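; BP_ButtonGreenhouse is a trigger that lets the player light a flame and open a linked door once LevelComplete is set on the character.
; On box overlap it points the character AnimBP's right-hand IK at DepressionFlame and plays a Timeline driving the IK alpha.
; Each Timeline update also shows the flame and calls OpenDoorWithButton on DoorSelect, with DoOnce guarding the match-lighting sound.
; Ending overlap reverses the Timeline.
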(event `self.Box.OnComponentBeginOverlap`
  (params (OverlappedComponent :type "PrimitiveComponent Object Reference") (OtherActor :type "Actor Object Reference") (OtherComp :type "PrimitiveComponent Object Reference") (OtherBodyIndex :type Integer) (bFromSweep :type Boolean) (SweepResult :type "HitResult Structure (by ref)"))
  (bind _asbp_third_person_character (cast `/Game/ThirdPerson/Blueprints/BP_ThirdPersonCharacter` OtherActor))
  (bind _levelcomplete (`/Game/ThirdPerson/Blueprints/BP_ThirdPersonCharacter.LevelComplete` _asbp_third_person_character))
  (if _levelcomplete
    (bind _asthird_person_anim_bp (cast `/Game/PolygonHorrorMansion/EpicContent/Mannequin/Animations/ThirdPerson_AnimBP` (`SkeletalMeshComponent.GetAnimInstance` (`Character.Mesh` _asbp_third_person_character))))
    (bind _output_get (set `self.AnimBP` _asthird_person_anim_bp))
    (set `/Game/PolygonHorrorMansion/EpicContent/Mannequin/Animations/ThirdPerson_AnimBP.RightHandIKTarget` (`SceneComponent.K2_GetComponentLocation` (`self.DepressionFlame`)) _output_get)
    (bind (_direction _newtrack_0) (`Timeline|Timeline` :!via `PlayFromStart` :!label _label)
      (:`Update`
        (set `/Game/PolygonHorrorMansion/EpicContent/Mannequin/Animations/ThirdPerson_AnimBP.RightHandIKAlpha` _newtrack_0 (`self.AnimBP`))
        (if _levelcomplete
          (`SceneComponent.SetVisibility` (`self.DepressionFlame`) true false)
          (`/Game/Blueprints/BP_DoorRightGreenhouse.OpenDoorWithButton` (`self.DoorSelect`))
          (`/Engine/EditorBlueprintResources/StandardMacros.DoOnce` false
            (:`Completed`
              (`GameplayStatics.PlaySoundAtLocation` "/Game/Audio/SFX_MatchLightingCandle.SFX_MatchLightingCandle" (0.0 0.0 0.0) (struct) 1.0 1.0 0.0 null null null null))))))))

(event `self.Box.OnComponentEndOverlap`
  (params (OverlappedComponent :type "PrimitiveComponent Object Reference") (OtherActor :type "Actor Object Reference") (OtherComp :type "PrimitiveComponent Object Reference") (OtherBodyIndex :type Integer))
  (goto _label :!via `Reverse`))

(fn `UserConstructionScript`)