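; BP_DestroyWall is a wall the third-person character can interact with and destroy, apparently using a hatchet.
; Its Box overlap registers the wall on the character as HatchetWall, enables wall interaction, and shows the Press E widget only if the character has a hatchet.
; Leaving the box clears that reference and flag and hides the prompt.
; A DestroyWall event, not called within this Blueprint, destroys the actor.
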(event `self.Box.OnComponentBeginOverlap`
  (params (OverlappedComponent :type "PrimitiveComponent Object Reference") (OtherActor :type "Actor Object Reference") (OtherComp :type "PrimitiveComponent Object Reference") (OtherBodyIndex :type Integer) (bFromSweep :type Boolean) (SweepResult :type "HitResult Structure (by ref)"))
  (bind _asbp_third_person_character (cast `/Game/ThirdPerson/Blueprints/BP_ThirdPersonCharacter` OtherActor))
  (set `/Game/ThirdPerson/Blueprints/BP_ThirdPersonCharacter.CanInteractWithWall` true _asbp_third_person_character)
  (set `/Game/ThirdPerson/Blueprints/BP_ThirdPersonCharacter.HatchetWall` self _asbp_third_person_character)
  (if (`/Game/ThirdPerson/Blueprints/BP_ThirdPersonCharacter.HasHatchet` _asbp_third_person_character)
    (`Widget.SetVisibility` (`/Game/ThirdPerson/Blueprints/BP_ThirdPersonCharacter.PressEWidget` _asbp_third_person_character) "Visible")))

(event `self.Box.OnComponentEndOverlap`
  (params (OverlappedComponent :type "PrimitiveComponent Object Reference") (OtherActor :type "Actor Object Reference") (OtherComp :type "PrimitiveComponent Object Reference") (OtherBodyIndex :type Integer))
  (bind _asbp_third_person_character (cast `/Game/ThirdPerson/Blueprints/BP_ThirdPersonCharacter` OtherActor))
  (set `/Game/ThirdPerson/Blueprints/BP_ThirdPersonCharacter.HatchetWall` null _asbp_third_person_character)
  (set `/Game/ThirdPerson/Blueprints/BP_ThirdPersonCharacter.CanInteractWithWall` false _asbp_third_person_character)
  (`Widget.SetVisibility` (`/Game/ThirdPerson/Blueprints/BP_ThirdPersonCharacter.PressEWidget` _asbp_third_person_character) "Hidden"))

(event `DestroyWall`
  (`self.K2_DestroyActor`))

(fn `UserConstructionScript`)